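; Player control Blueprint for a chess game that turns left mouse clicks into board clicks.
; On BeginPlay it shows the cursor and caches the first BP_ChessBoard in the level.
; Each click traces under the cursor on the Visibility channel and passes the hit location to the board's Click.
; Its own Click function, not called here, prints the grid cell of a position using 400-unit squares.
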(event EventBeginPlay
  (Variables|/Script/Engine.PlayerController|SetbShowMouseCursor (Game|GetPlayerController 0) true)
  (bind _outactors (Actor|GetAllActorsOfClass "/Game/Esset/01_BluePrints/BP_ChessBoard.BP_ChessBoard_C"))
  (bind _asbp_chess_board (Utilities|Casting|CastToBP_ChessBoard (Utilities|Array|Get(acopy) _outactors)))
  (Variables|Default|SetChessBoard_C _asbp_chess_board))

(event EventTick
  (params (DeltaSeconds :type Float%20%28single-precision%29)))

(event Input|MouseEvents|LeftMouseButton
  (params (Key :type Key%20Structure :default "None"))
  (:Pressed
    (Default|Click (Variables|Default|GetChessBoard_C) (.Location (Collision|BreakHitResult (.HitResult (Game|Player|GetHitResultUnderCursorbyChannel "TraceTypeQuery1" true)))))))

(fn ConstructionScript)

(fn Click
  (params (Position :type Vector))
  (bind _returnvalue (/ Position "400.000000,400.000000,1.000000"))
  (bind (_x _y) (Math|Vector|BreakVector _returnvalue))
  (Development|PrintString (Utilities|String|BuildString(Integer) (Utilities|String|ToString(Integer) (Math|Float|Floor _x)) "" (Math|Float|Floor _y))))