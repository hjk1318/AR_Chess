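; BP_ChessBoard is an actor that builds an 8x8 chessboard with pieces and handles first-click square highlighting.
; The construction script generates checkered square meshes and piece meshes chosen from StartFigures, colored by board half, caching components in arrays.
; Click converts a position to a square index, turns that square gold and stores it in LastClick, only when none is selected.
; No move logic exists yet, and the event graph is empty.
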(event EventBeginPlay)

(event Collision|EventActorBeginOverlap
  (params (OtherActor :type Actor%20Object%20Reference)))

(event EventTick
  (params (DeltaSeconds :type Float%20%28single-precision%29)))

(fn ConstructionScript
  ;[1 1 1] 스태틱 메쉬를 메테리얼을 부여해서 생성하는 식
  (for _index (range 0 63)
    (Utilities|FlowControl|Sequence
      (:then_0
        (bind _returnvalue (AddComponent|AddStaticMeshComponent false (Math|Conversions|ToTransform(Vector) (Math|Vector|MakeVector (Math|Conversions|ToFloat(Integer) (* (/ _index 8) 400)) (Math|Conversions|ToFloat(Integer) (* (Math|Integer|%(Integer) _index 8) 400)) 0.0))))
        (Utilities|Array|Add (Variables|Default|GetFileds_Mesh) _returnvalue)
        (Rendering|Material|SetMaterial _returnvalue 0 (select (Class|KismetMathLibrary|XORBoolean (Math|Conversions|ToBoolean(Integer) (Math|Integer|%(Integer) _index 2)) (Math|Conversions|ToBoolean(Integer) (Math|Integer|%(Integer) (/ _index 8) 2))) "/Game/Esset/03_Material/M_Basic_BlackCheker.M_Basic_BlackCheker" "/Game/Esset/03_Material/M_Basic_WhiteCheker.M_Basic_WhiteCheker"))
        (Utilities|Array|Add (Variables|Default|GetFileds_Material) (select (Class|KismetMathLibrary|XORBoolean (Math|Conversions|ToBoolean(Integer) (Math|Integer|%(Integer) _index 2)) (Math|Conversions|ToBoolean(Integer) (Math|Integer|%(Integer) (/ _index 8) 2))) "/Game/Esset/03_Material/M_Basic_BlackCheker.M_Basic_BlackCheker" "/Game/Esset/03_Material/M_Basic_WhiteCheker.M_Basic_WhiteCheker")))
      (:then_1
        ;[1 1 1] 체스 피스 배치
        (bind _returnvalue_2 (AddComponent|AddStaticMeshComponent false (Math|Conversions|ToTransform(Vector) (+ (Math|Vector|MakeVector (Math|Conversions|ToFloat(Integer) (* (/ _index 8) 400)) (Math|Conversions|ToFloat(Integer) (* (Math|Integer|%(Integer) _index 8) 400)) 0.0) "200.000000,200.000000,0.000000"))))
        (Components|StaticMesh|SetStaticMesh _returnvalue_2 (Utilities|Select :Index (Utilities|Array|Get(acopy) (Variables|Default|GetStart_Figures) _index) :Option%200 0 :Option%201 "/Game/Esset/05_Model/Test_chess_piece/Pawn.Pawn" :Option%202 "/Game/Esset/05_Model/Test_chess_piece/Rook.Rook" :Option%203 "/Game/Esset/05_Model/Test_chess_piece/Knight.Knight" :Option%204 "/Game/Esset/05_Model/Test_chess_piece/Bishop.Bishop" :Option%205 "/Game/Esset/05_Model/Test_chess_piece/Queen.Queen" :Option%206 "/Game/Esset/05_Model/Test_chess_piece/King.King"))
        (Rendering|Material|SetMaterial _returnvalue_2 0 (select (> _index 30) "/Game/Esset/03_Material/M_Basic_WhiteCheker.M_Basic_WhiteCheker" "/Game/Esset/03_Material/M_Basic_BlackCheker.M_Basic_BlackCheker"))
        (Utilities|Array|Add (Variables|Default|Getpiecies_Mesh) _returnvalue_2)))))

(fn Click
  (params (position :type Vector))
  (bind _returnvalue (Utilities|Position->Index position))
  (if (== (Variables|Default|GetLast_Click) -1)
    (Rendering|Material|SetMaterial (Utilities|Array|Get(acopy) (Variables|Default|GetFileds_Mesh) _returnvalue) 0 "/Game/StarterContent/Materials/M_Metal_Gold.M_Metal_Gold")
    (Variables|Default|SetLast_Click _returnvalue)))